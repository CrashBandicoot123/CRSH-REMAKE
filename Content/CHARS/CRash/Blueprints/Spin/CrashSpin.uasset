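; CrashSpin is Crash Bandicoot's spin attack, a weapon-style Blueprint triggered by the SPin input action.
; BeginPlay caches the player character, and each press plays the spin animation on the skeletal mesh.
; It then runs a debug-drawn multi-sphere trace forward from the character, using the range in WeaponInfo.
; Each hit gets the VFX, sound and damage defined in WeaponInfo.
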(event EventBeginPlay
  (bind _ascrashbandicoot (Utilities|Casting|CastToCRASHBANDICOOT (Game|GetPlayerCharacter 0)))
  (Variables|Default|SetCharacter%20Reference _ascrashbandicoot))

(event Input|ActionEvents|InputActionSPin
  (params (Key :type Key%20Structure :default "AnyKey"))
  (bind _character_reference (Variables|Default|GetCharacter%20Reference))
  (bind _weaponinfo (Variables|Default|GetWeaponInfo))
  (bind (_damage _range _attackvfx _attacksfx _hitvfx _hitsfx) (Utilities|Struct|BreakAttackInfo _weaponinfo))
  (bind _returnvalue (Transformation|GetActorLocation _character_reference))
  (:Pressed
    (Components|Animation|PlayAnimation (Variables|Default|GetSkeletalMesh) "/Game/CHARS/CRash/CrashSpin/CrashSpin_Anim_Armature_Spin.CrashSpin_Anim_Armature_Spin" false)
    (bind (_outhits _returnvalue_2) (Collision|MultiSphereTraceByChannel _returnvalue (+ _returnvalue (* (Transformation|GetActorForwardVector _character_reference) (.range (Variables|Default|GetWeaponInfo)))) 0.0 "TraceTypeQuery2" false (Utilities|Array|MakeArray _character_reference) "ForDuration"))
    (if _returnvalue_2
      (for _array_element _outhits
        (Effects|SpawnEmitteratLocation _hitvfx (.Location (Collision|BreakHitResult _array_element)))
        (Audio|PlaySoundatLocation _hitsfx (.Location (Collision|BreakHitResult _array_element)))
        (Game|Damage|ApplyDamage (.HitActor (Collision|BreakHitResult _array_element)) _damage 0 (Variables|Default|GetCharacter%20Reference))))))

(fn ConstructionScript)
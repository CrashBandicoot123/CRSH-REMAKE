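; TNT crate for the Crash Bandicoot character that counts down after an overlap, then vanishes in fire smoke.
; Initiator overlap casts player 0 without checking the overlapping actor; its jump-collider condition uses a constructed hit result, so always passes.
; A Delay chain swaps countdown materials with tick sounds each second, then destroys the crate and spawns the emitter.
; Any damage destroys it immediately without effects; neither path applies damage.
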(event OnComponentBeginOverlap(Initiator)
  (params (OverlappedComponent :type Primitive%20Component%20Object%20Reference) (OtherActor :type Actor%20Object%20Reference) (OtherComp :type Primitive%20Component%20Object%20Reference) (OtherBodyIndex :type Integer) (bFromSweep :type Boolean) (SweepResult :type Hit%20Result%20Structure%20%28by%20ref%29))
  (bind _self self)
  (bind _ascrashbandicoot (Utilities|Casting|CastToCRASHBANDICOOT (Game|GetPlayerCharacter 0)))
  (if (.bInitialOverlap (Collision|BreakHitResult (Collision|MakeHitResult false true 0.0 "0, 0, 0" "0, 0, 0" "0,0,1" "0,0,1" 0 _self (Variables|/Game/CHARS/CRash/Blueprints/CRASHBANDICOOT.CRASHBANDICOOT_C|GetJumpColliderCrash _ascrashbandicoot))))
    (Audio|SpawnSound2D "/Game/Sound/SFX/Bounce.Bounce")
    (Audio|SpawnSound2D "/Game/Sound/SFX/BombTick.BombTick")
    (Rendering|Material|SetMaterial (Variables|Default|GetStaticMesh) 1 "/Game/Collectibles/Box/TNT/tnt_countdown_3_Mat.tnt_countdown_3_Mat")
    (Utilities|FlowControl|Delay 1.0)
    (Audio|SpawnSound2D "/Game/Sound/SFX/BombTick.BombTick")
    (Rendering|Material|SetMaterial (Variables|Default|GetStaticMesh) 1 "/Game/Collectibles/Box/TNT/tnt_countdown_2_Mat.tnt_countdown_2_Mat")
    (Utilities|FlowControl|Delay 1.0)
    (Audio|SpawnSound2D "/Game/Sound/SFX/BombTick.BombTick")
    (Rendering|Material|SetMaterial (Variables|Default|GetStaticMesh) 1 "/Game/Collectibles/Box/TNT/tnt_countdown_1_Mat.tnt_countdown_1_Mat")
    (Utilities|FlowControl|Delay 1.0)
    (Actor|DestroyActor _self)
    (Effects|SpawnEmitteratLocation "/Game/Particles/Fire/FireSmoke.FireSmoke" "0, 0, 0")))

(event Game|Damage|EventAnyDamage
  (params (Damage :type Float%20%28single-precision%29) (DamageType :type Damage%20Type%20Object%20Reference) (InstigatedBy :type Controller%20Object%20Reference) (DamageCauser :type Actor%20Object%20Reference))
  (Actor|DestroyActor self))

(fn ConstructionScript)
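; AkuCrate is a collectible crate that awards Crash an Aku when his jump collider overlaps it.
; At BeginPlay it searches for CRASHBANDICOOT actors and caches the last one found along with its JumpColliderCrash.
; An overlap between that collider and the crate's JumpCollider plays the Aku sound, increments Crash's Akus count, launches him upward and destroys the crate.
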(event OnComponentBeginOverlap(JumpCollider)
  (params (OverlappedComponent :type Primitive%20Component%20Object%20Reference) (OtherActor :type Actor%20Object%20Reference) (OtherComp :type Primitive%20Component%20Object%20Reference) (OtherBodyIndex :type Integer) (bFromSweep :type Boolean) (SweepResult :type Hit%20Result%20Structure%20%28by%20ref%29))
  (bind _crash (Variables|Default|GetCrash))
  (if (== OtherComp (Variables|Default|GetCrashCollider))
    (bind _ascrashbandicoot (Utilities|Casting|CastToCRASHBANDICOOT _crash))
    (Audio|PlaySoundatLocation (Variables|Default|GetAkuSound) (Transformation|GetActorLocation _crash))
    (Variables|/Game/CHARS/CRash/Blueprints/CRASHBANDICOOT.CRASHBANDICOOT_C|SetAkus _ascrashbandicoot (+ (Variables|/Game/CHARS/CRash/Blueprints/CRASHBANDICOOT.CRASHBANDICOOT_C|GetAkus _ascrashbandicoot) 1))
    (Character|LaunchCharacter _ascrashbandicoot "0, 0,2000.000000" false false)
    (Actor|DestroyActor)))

(event EventBeginPlay
  (bind _outactors (Actor|GetAllActorsOfClass "/Game/CHARS/CRash/Blueprints/CRASHBANDICOOT.CRASHBANDICOOT_C"))
  (for _array_element _outactors
    _)
  (Variables|Default|SetCrashCollider (Variables|/Game/CHARS/CRash/Blueprints/CRASHBANDICOOT.CRASHBANDICOOT_C|GetJumpColliderCrash _array_element))
  (Variables|Default|SetCrash _array_element))

(fn ConstructionScript)
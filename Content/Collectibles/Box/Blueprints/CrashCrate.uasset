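; Crash Bandicoot collectible crate that grants the player one extra life and destroys itself when damaged or jumped on.
; Any damage to the crate awards the life directly, while a Box overlap also plays a bounce sound and launches Crash upward.
; Both events cast player character 0 to CRASHBANDICOOT without checking which actor caused the damage or overlap.
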(event OnComponentBeginOverlap(Box)
  (params (OverlappedComponent :type Primitive%20Component%20Object%20Reference) (OtherActor :type Actor%20Object%20Reference) (OtherComp :type Primitive%20Component%20Object%20Reference) (OtherBodyIndex :type Integer) (bFromSweep :type Boolean) (SweepResult :type Hit%20Result%20Structure%20%28by%20ref%29))
  ;[1 1 1] When Crash is Jumping on The crate
  (bind _ascrashbandicoot (Utilities|Casting|CastToCRASHBANDICOOT (Game|GetPlayerCharacter 0)))
  (Audio|PlaySoundatLocation "/Game/Sound/SFX/Bounce.Bounce" (Transformation|GetActorLocation self))
  (Variables|/Game/CHARS/CRash/Blueprints/CRASHBANDICOOT.CRASHBANDICOOT_C|SetLives _ascrashbandicoot (+ (Variables|/Game/CHARS/CRash/Blueprints/CRASHBANDICOOT.CRASHBANDICOOT_C|GetLives _ascrashbandicoot) 1))
  (Character|LaunchCharacter _ascrashbandicoot "0, 0,2000.000000" false false)
  (Actor|DestroyActor self))

(event Game|Damage|EventAnyDamage
  (params (Damage :type Float%20%28single-precision%29) (DamageType :type Damage%20Type%20Object%20Reference) (InstigatedBy :type Controller%20Object%20Reference) (DamageCauser :type Actor%20Object%20Reference))
  ;[1 1 1] If Crash Damages instead of Jumping on the Crate
  (bind _ascrashbandicoot (Utilities|Casting|CastToCRASHBANDICOOT (Game|GetPlayerCharacter 0)))
  (Variables|/Game/CHARS/CRash/Blueprints/CRASHBANDICOOT.CRASHBANDICOOT_C|SetLives _ascrashbandicoot (+ (Variables|/Game/CHARS/CRash/Blueprints/CRASHBANDICOOT.CRASHBANDICOOT_C|GetLives _ascrashbandicoot) 1))
  (Actor|DestroyActor self))

(fn ConstructionScript)
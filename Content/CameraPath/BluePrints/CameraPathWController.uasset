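; Spline camera path actor that takes over the player's view when the player overlaps an activating endpoint, and can restore the previous camera.
; Sampled spline checkpoints let the spring arm ease toward the one nearest the target, or it travels the spline cinematically and deactivates at the end.
; Rotation tracks the target with clamped pitch, also setting control rotation, or follows the spline.
; The construction script positions endpoints and draws direction arrows along the path.
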(event OnComponentBeginOverlap(Endpoint1)
  (params (OverlappedComponent :type Primitive%20Component%20Object%20Reference) (OtherActor :type Actor%20Object%20Reference) (OtherComp :type Primitive%20Component%20Object%20Reference) (OtherBodyIndex :type Integer) (bFromSweep :type Boolean) (SweepResult :type Hit%20Result%20Structure%20%28by%20ref%29))
  ;[1 1 1] Overlap endpoints: If either of the endpoints is set to activate the camera (at least one of these needs to be on to work properly), otherwise return to the previous camera if it exists
  (Variables|Targeting|SetTarget OtherActor)
  (if (and (Variables|Endpoints|GetEndpoint1Activates) (== OtherActor (Game|Player|GetPlayerPawn 0)))
    (if (not (Components|Activation|IsActive (Variables|Default|GetCamera)))
      (bind _outactors (Actor|GetAllActorsOfClass "/Script/Engine.CameraActor"))
      (for _array_element _outactors
        (if (Components|Activation|IsActive (Variables|/Script/Engine.CameraActor|GetCameraComponent _array_element))
          (Variables|Camera|SetLastCamera _array_element)
          (Components|Activation|Deactivate (Variables|/Script/Engine.CameraActor|GetCameraComponent _array_element))))
      (Components|Activation|Activate (Variables|Default|GetCamera) false)
      (Game|Player|SetViewTargetwithBlend (Game|GetPlayerController 0) self 0.1 "VTBlend_Cubic" 0.0 false))
    (elif (!= (Variables|Camera|GetLastCamera) 0)
      (Components|Activation|Activate (Variables|/Script/Engine.CameraActor|GetCameraComponent (Variables|Camera|GetLastCamera)) false)
      (Game|Player|SetViewTargetwithBlend (Game|GetPlayerController 0) (Variables|Camera|GetLastCamera) 0.5 "VTBlend_Cubic" 0.0 false)
      (Components|Activation|Deactivate (Variables|Default|GetCamera)))))

(event OnComponentBeginOverlap(Endpoint2)
  (params (OverlappedComponent :type Primitive%20Component%20Object%20Reference) (OtherActor :type Actor%20Object%20Reference) (OtherComp :type Primitive%20Component%20Object%20Reference) (OtherBodyIndex :type Integer) (bFromSweep :type Boolean) (SweepResult :type Hit%20Result%20Structure%20%28by%20ref%29))
  ;[1 1 1] Overlap endpoints: If either of the endpoints is set to activate the camera (at least one of these needs to be on to work properly), otherwise return to the previous camera if it exists
  (Variables|Targeting|SetTarget OtherActor)
  (if (and (Variables|Endpoints|GetEndpoint2Activates) (== OtherActor (Game|Player|GetPlayerPawn 0)))
    (if (not (Components|Activation|IsActive (Variables|Default|GetCamera)))
      (bind _outactors (Actor|GetAllActorsOfClass "/Script/Engine.CameraActor"))
      (for _array_element _outactors
        (if (Components|Activation|IsActive (Variables|/Script/Engine.CameraActor|GetCameraComponent _array_element))
          (Variables|Camera|SetLastCamera _array_element)
          (Components|Activation|Deactivate (Variables|/Script/Engine.CameraActor|GetCameraComponent _array_element))))
      (Components|Activation|Activate (Variables|Default|GetCamera) false)
      (Game|Player|SetViewTargetwithBlend (Game|GetPlayerController 0) self 0.1 "VTBlend_Cubic" 0.0 false))
    (elif (!= (Variables|Camera|GetLastCamera) 0)
      (Components|Activation|Activate (Variables|/Script/Engine.CameraActor|GetCameraComponent (Variables|Camera|GetLastCamera)) false)
      (Game|Player|SetViewTargetwithBlend (Game|GetPlayerController 0) (Variables|Camera|GetLastCamera) 0.5 "VTBlend_Cubic" 0.0 false)
      (Components|Activation|Deactivate (Variables|Default|GetCamera)))))

(event Custom|Activate_Event
  ;[1 1 1] Overlap endpoints: If either of the endpoints is set to activate the camera (at least one of these needs to be on to work properly), otherwise return to the previous camera if it exists
  (if (not (Components|Activation|IsActive (Variables|Default|GetCamera)))
    (bind _outactors (Actor|GetAllActorsOfClass "/Script/Engine.CameraActor"))
    (for _array_element _outactors
      (if (Components|Activation|IsActive (Variables|/Script/Engine.CameraActor|GetCameraComponent _array_element))
        (Variables|Camera|SetLastCamera _array_element)
        (Components|Activation|Deactivate (Variables|/Script/Engine.CameraActor|GetCameraComponent _array_element))))
    (Components|Activation|Activate (Variables|Default|GetCamera) false)
    (Game|Player|SetViewTargetwithBlend (Game|GetPlayerController 0) self 0.1 "VTBlend_Cubic" 0.0 false)))

(event Custom|Deactivate_Event
  (bind _lastcamera (Variables|Camera|GetLastCamera))
  ;[1 1 1] Overlap endpoints: If either of the endpoints is set to activate the camera (at least one of these needs to be on to work properly), otherwise return to the previous camera if it exists
  (if (!= _lastcamera 0)
    (Components|Activation|Activate (Variables|/Script/Engine.CameraActor|GetCameraComponent _lastcamera) false)
    (Game|Player|SetViewTargetwithBlend (Game|GetPlayerController 0) (Variables|Camera|GetLastCamera) 0.5 "VTBlend_Cubic" 0.0 false)
    (Components|Activation|Deactivate (Variables|Default|GetCamera))))

(event EventBeginPlay
  (bind _path (Variables|Default|GetPath))
  (Components|Activation|Deactivate (Variables|Default|GetCamera))
  ;[1 1 1] BeginPlay: When play begins we want to make the checkpoints fresh
  ;;[1 1 1] Freshen up our arrays of transforms (Checkpoints)
  (Variables|Checkpoints|SetUpdatePath true)
  (Utilities|Array|Clear (Variables|Checkpoints|GetCheckPointsRelative))
  (Utilities|Array|Clear (Variables|Checkpoints|GetCheckPointsWorld))
  (Variables|Checkpoints|SetSplineStep (/ (Spline|GetSplineLength (Variables|Default|GetPath)) (Math|Conversions|ToFloat(Integer) (Variables|Checkpoints|GetCheckpointDensity))))
  (for _index (range 0 (Variables|Checkpoints|GetCheckpointDensity))
    ;;[1 1 1] Fill our checkpoint arrays with all the transforms along the path, these are used both to check against player location as well as moving the camera
    (Utilities|Array|Add (Variables|Checkpoints|GetCheckPointsRelative) (Spline|GetTransformatDistanceAlongSpline _path (* _index (Variables|Checkpoints|GetSplineStep)) "Local" false))
    (Utilities|Array|Add (Variables|Checkpoints|GetCheckPointsWorld) (Spline|GetTransformatDistanceAlongSpline _path (* _index (Variables|Checkpoints|GetSplineStep)) "World" false))))

(event EventTick
  (params (DeltaSeconds :type Float%20%28single-precision%29))
  (bind _springarm (Variables|Default|GetSpringArm))
  (bind _springarm_2 (Variables|Default|GetSpringArm))
  ;[1 1 1] Tick if this camera is the active one
  (Variables|Default|SetDeltaTime DeltaSeconds)
  (if (Components|Activation|IsActive (Variables|Default|GetCamera))
    (Utilities|FlowControl|Sequence
      (:then_0
        ;[1 1 1] Translation
        (if (Variables|Targeting|GetFollowTarget)
          ;;[1 1 1] Find the closest checkpoint then move the camera toward it
          (Variables|Targeting|SetDistanceToTarget 1e+39)
          (Variables|Checkpoints|SetCurrentCheckPoint 1)
          (for (_array_element _array_index) (Variables|Checkpoints|GetCheckPointsWorld)
            (if (< (Math|Vector|VectorLength (- (.Location (Math|Transform|BreakTransform _array_element)) (Transformation|GetActorLocation (Variables|Targeting|GetTarget)))) (Variables|Targeting|GetDistanceToTarget))
              (Variables|Checkpoints|SetCurrentCheckPoint _array_index)
              (Variables|Targeting|SetDistanceToTarget (Math|Vector|VectorLength (- (.Location (Math|Transform|BreakTransform _array_element)) (Transformation|GetActorLocation (Variables|Targeting|GetTarget)))))))
          (Transformation|SetWorldLocation _springarm (Math|Interpolation|VInterpTo (Transformation|GetWorldLocation _springarm) (.Location (Math|Transform|BreakTransform (Utilities|Array|Get(acopy) (Variables|Checkpoints|GetCheckPointsWorld) (Variables|Checkpoints|GetCurrentCheckPoint)))) (Variables|Default|GetDeltaTime) (Variables|Camera|GetTranslateSpeed)) false false)
          (else
            ;;[1 1 1] Move along the spline smoothly if we aren't following target location
            (bind _output_get (Variables|Camera|SetDistanceAlongSpline (+ (Variables|Camera|GetDistanceAlongSpline) (* (Variables|Camera|GetTranslateSpeed) (Variables|Default|GetDeltaTime) (Variables|Camera|GetCinematicSpeedScale)))))
            (if (>= _output_get (Spline|GetSplineLength (Variables|Default|GetPath)))
              (Variables|Camera|SetDistanceAlongSpline 1.0)
              (CallFunction|DeactivateEvent)
              (else
                (Transformation|SetWorldLocation (Variables|Default|GetSpringArm) (Spline|GetLocationatDistanceAlongSpline (Variables|Default|GetPath) (Variables|Camera|GetDistanceAlongSpline) "World") false false))))))
      (:then_1
        ;[1 1 1] Rotation
        (if (and (Variables|Targeting|GetAlwaysLookAtTarget) (!= (Variables|Targeting|GetTarget) 0))
          ;;[1 1 1] If we have a target, and AlwaysLookAtTarget is true, then rotate based on look at direction to target
          (Transformation|SetWorldRotation _springarm_2 (Math|Rotator|MakeRotator 0.0 (+ (Math|Float|ClampAngle (- (.Pitch (Math|Rotator|BreakRotator (Math|Interpolation|RInterpTo (Transformation|GetWorldRotation _springarm_2) (Math|Rotator|FindLookatRotation (Transformation|GetWorldLocation _springarm_2) (Transformation|GetActorLocation (Variables|Targeting|GetTarget))) (Variables|Default|GetDeltaTime) (Variables|Camera|GetRotationSpeed)))) 1.8e+02) 1.5e+02 -125.0) 1.8e+02) (.Yaw (Math|Rotator|BreakRotator (Math|Interpolation|RInterpTo (Transformation|GetWorldRotation _springarm_2) (Math|Rotator|FindLookatRotation (Transformation|GetWorldLocation _springarm_2) (Transformation|GetActorLocation (Variables|Targeting|GetTarget))) (Variables|Default|GetDeltaTime) (Variables|Camera|GetRotationSpeed))))) false false)
          (Pawn|SetControlRotation (Game|GetPlayerController 0) (Math|Rotator|MakeRotator 0.0 (+ (Math|Float|ClampAngle (- (.Pitch (Math|Rotator|BreakRotator (Math|Interpolation|RInterpTo (Transformation|GetWorldRotation _springarm_2) (Math|Rotator|FindLookatRotation (Transformation|GetWorldLocation _springarm_2) (Transformation|GetActorLocation (Variables|Targeting|GetTarget))) (Variables|Default|GetDeltaTime) (Variables|Camera|GetRotationSpeed)))) 1.8e+02) 1.5e+02 -125.0) 1.8e+02) (.Yaw (Math|Rotator|BreakRotator (Math|Interpolation|RInterpTo (Transformation|GetWorldRotation _springarm_2) (Math|Rotator|FindLookatRotation (Transformation|GetWorldLocation _springarm_2) (Transformation|GetActorLocation (Variables|Targeting|GetTarget))) (Variables|Default|GetDeltaTime) (Variables|Camera|GetRotationSpeed))))))
          (else
            (Transformation|SetWorldRotation (Variables|Default|GetSpringArm) (Spline|GetRotationatDistanceAlongSpline (Variables|Default|GetPath) (Variables|Camera|GetDistanceAlongSpline) "Local") false false)))))))

(fn ConstructionScript
  (bind _path (Variables|Default|GetPath))
  (Components|Activation|Deactivate (Variables|Default|GetCamera))
  (Transformation|SetWorldTransform (Variables|Default|GetSpringArm) (Spline|GetTransformatDistanceAlongSpline (Variables|Default|GetPath) 0.0 "World" false) false false)
  ;[1 1 1] When first placed, or if it needs reseting for some odd reason, move the transform widgets back to the endpoint boxes
  (if (Variables|Endpoints|GetResetEndpoints)
    (Variables|Endpoints|SetResetEndpoints false)
    (Variables|Endpoints|SetEndpoint1Transform (Transformation|GetRelativeTransform (Variables|Default|GetEndpoint1)))
    (Variables|Endpoints|SetEndpoint2Transform (Transformation|GetRelativeTransform (Variables|Default|GetEndpoint2)))
    (else
      ;[1 1 1] Otherwise move the endpoints to the proper transform locations
      (Transformation|SetRelativeTransform (Variables|Default|GetEndpoint1) (Variables|Endpoints|GetEndpoint1Transform) false false)
      (Transformation|SetRelativeTransform (Variables|Default|GetEndpoint2) (Variables|Endpoints|GetEndpoint2Transform) false false)))
  ;[1 1 1] We don't want to update our path everytime it's touched, that gets crazy resource intensive
  (if (Variables|Checkpoints|GetUpdatePath)
    ;[1 1 1] Freshen up our arrays of transforms (Checkpoints)
    (Variables|Checkpoints|SetUpdatePath true)
    (Utilities|Array|Clear (Variables|Checkpoints|GetCheckPointsRelative))
    (Utilities|Array|Clear (Variables|Checkpoints|GetCheckPointsWorld))
    (Variables|Checkpoints|SetSplineStep (/ (Spline|GetSplineLength (Variables|Default|GetPath)) (Math|Conversions|ToFloat(Integer) (Variables|Checkpoints|GetCheckpointDensity))))
    (for _index (range 0 (Variables|Checkpoints|GetCheckpointDensity))
      ;[1 1 1] Fill our checkpoint arrays with all the transforms along the path, these are used both to check against player location as well as moving the camera
      (Utilities|Array|Add (Variables|Checkpoints|GetCheckPointsRelative) (Spline|GetTransformatDistanceAlongSpline _path (* _index (Variables|Checkpoints|GetSplineStep)) "Local" false))
      (Utilities|Array|Add (Variables|Checkpoints|GetCheckPointsWorld) (Spline|GetTransformatDistanceAlongSpline _path (* _index (Variables|Checkpoints|GetSplineStep)) "World" false)))
    ;[1 1 1] Add arrows for visualizing the direction that the camera will face while traveling along the path
    (for _index_2 (range 0 (Variables|Checkpoints|GetCheckpointDensity))
      (bind _returnvalue (AddComponent|AddArrowComponent true (Utilities|Array|Get(acopy) (Variables|Checkpoints|GetCheckPointsRelative) _index_2)))
      (Transformation|AttachComponentToComponent _returnvalue (Variables|Default|GetPath) "None" "KeepWorld" "KeepWorld" "KeepWorld" false)
      (if (== (.Remainder (Math|Float|Division(WholeandRemainder) (Math|Conversions|ToFloat(Integer) _index_2) 5.0)) 0.0)
        (Transformation|SetWorldScale3D _returnvalue "4.000000,4.000000,4.000000")
        (else
          (Transformation|SetWorldScale3D _returnvalue "2.000000,2.000000,2.000000"))))))